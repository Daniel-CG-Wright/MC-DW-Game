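; First-person player character Blueprint that puts a HUD on screen, handles crouching and landing, and can spawn and equip a prototype pistol.
; A timeline lerps the capsule half-height between standing and crouched, supporting hold or toggle crouch via PressCrouch and ReleaseCrouch.
; Landing drops walk speed to crouch speed until a timer calls "Speed back up" by name to restore the default.
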(event `self.ReceiveBeginPlay`
  (bind _returnvalue (`|CreateWidget` "/Game/Blueprints/UI/HUD.HUD_C"))
  (bind _output_get (set `self.HUD reference` _returnvalue))
  (`UserWidget.AddToViewport` _output_get 0))

(event `self.OnLanded`
  (params (Hit :type "HitResult Structure (by ref)"))
  (set `self.JustLanded` true)
  (set `CharacterMovementComponent.MaxWalkSpeed` (`self.CrouchSpeed`) (`self.CharacterMovement`))
  (`KismetSystemLibrary.K2_SetTimer` null "Speed back up" (`self.LandingTime`)))

(event `InputAction|Crouch`
  (params (Key :type "Key Structure"))
  ;[1 1 1] Crouch
  (:`Pressed`
    (`self.PressCrouch`)
    (if (`self.CurrentlyCrouching`)
      (bind (_direction _crouch) (`Timeline|Timeline_Crouch` :!label _label)
        (:`Update`
          (`CapsuleComponent.SetCapsuleHalfHeight` (`self.CapsuleComponent`) (`KismetMathLibrary.Lerp` (`self.DefaultHalfHeight`) (`self.CrouchedHalfHeight`) _crouch) true)))
      (else
        (goto _label :!via `Reverse`))))
  (:`Released`
    (`self.ReleaseCrouch`)
    (if (not (`self.ToggleCrouch`))
      (goto _label :!via `Reverse`))))

(event `self.SpawnAndEquipGun`
  (bind _returnvalue (`|SpawnActorFromClass` "/Game/Blueprints/Weapons/BP_PrototypePistol.BP_PrototypePistol_C" (`self.GetTransform`) "Undefined" "OverrideRootScale" null null))
  (`self.EquipWeapon` _returnvalue))

(fn `Speed back up`
  (set `self.JustLanded` false)
  (set `CharacterMovementComponent.MaxWalkSpeed` (`self.DefaultSpeed`) (`self.CharacterMovement`)))

(fn `UserConstructionScript`)