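; First-person character Blueprint with networked crouching, a landing slowdown and a HUD created on non-authority instances.
; Crouch input supports toggle or hold, gates standing up on CanUncrouch, and forwards the state from clients to the server.
; Timelines blend capsule half-height alongside walk-speed changes, mirrored in the CurrentlyCrouching rep-notify.
; Landing drops speed to CrouchSpeed until a LandingTime timer restores DefaultSpeed.
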(event `self.ReceiveBeginPlay`
  (if (not (`self.HasAuthority`))
    (bind _returnvalue (`|CreateWidget` "/Game/Blueprints/UI/HUD.HUD_C"))
    (bind _output_get (set `self.HUD reference` _returnvalue))
    (`UserWidget.AddToViewport` _output_get 0)))

(event `self.OnLanded`
  (params (Hit :type "HitResult Structure (by ref)"))
  (set `self.JustLanded` true)
  (set `CharacterMovementComponent.MaxWalkSpeed` (`self.CrouchSpeed`) (`self.CharacterMovement`))
  (`KismetSystemLibrary.K2_SetTimer` null "Speed back up" (`self.LandingTime`)))

(event `ServerSetCrouch`
  (params (NewCrouch :type Boolean))
  ;[1 1 1] Crouching code
  (`self.SetCrouch` NewCrouch))

(event `SetCrouch`
  (params (NewCrouch :type Boolean))
  (bind _charactermovement (`self.CharacterMovement`))
  (if NewCrouch
    ;[1 1 1] Crouching code
    (if (not (`self.HasAuthority`)) :!label _label
      (`self.ServerSetCrouch` NewCrouch))
    (bind _output_get (set `self.CurrentlyCrouching` NewCrouch))
    (if _output_get
      (set `CharacterMovementComponent.MaxWalkSpeed` (`self.CrouchSpeed`) _charactermovement)
      (else
        (set `CharacterMovementComponent.MaxWalkSpeed` (`self.DefaultSpeed`) _charactermovement)))
    (if (`self.CurrentlyCrouching`)
      (bind (_direction _crouch) (`Timeline|Timeline_0` :!label _label_2)
        (:`Update`
          (`CapsuleComponent.SetCapsuleHalfHeight` (`self.CapsuleComponent`) (`KismetMathLibrary.Lerp` (`self.DefaultHalfHeight`) (`self.CrouchedHalfHeight`) _crouch) true)))
      (else
        (goto _label_2 :!via `Reverse`)))
    (else
      (bind _returnvalue (`self.CanUncrouch`))
      (if _returnvalue
        (goto _label)))))

(event `InputAction|Crouch`
  (params (Key :type "Key Structure"))
  ;[1 1 1] Crouching code
  (:`Pressed`
    (if (`self.ToggleCrouch`)
      (if (`self.CurrentlyCrouching`)
        (`self.SetCrouch` false)
        (else
          (`self.SetCrouch` true)))
      (else
        (`self.SetCrouch` true))))
  (:`Released`
    (if (not (`self.ToggleCrouch`))
      (`self.SetCrouch` false))))

(event `self.BlueprintRep_CurrentlyCrouching`
  (bind _charactermovement (`self.CharacterMovement`))
  (bind _currentlycrouching (`self.CurrentlyCrouching`))
  (if _currentlycrouching
    (set `CharacterMovementComponent.MaxWalkSpeed` (`self.CrouchSpeed`) _charactermovement)
    (else
      (set `CharacterMovementComponent.MaxWalkSpeed` (`self.DefaultSpeed`) _charactermovement)))
  (if _currentlycrouching
    (bind (_direction _crouch) (`Timeline|Timeline_1` :!label _label_3)
      (:`Update`
        (`CapsuleComponent.SetCapsuleHalfHeight` (`self.CapsuleComponent`) (`KismetMathLibrary.Lerp` (`self.DefaultHalfHeight`) (`self.CrouchedHalfHeight`) _crouch) true)))
    (else
      (goto _label_3 :!via `Reverse`))))

(fn `Get Synchronised Control Rotation`
  (returns (`sync rotation` :type "Rotator Structure"))
  (return (`self.SynchronisedControlRotation`)))

(fn `Speed back up`
  (set `self.JustLanded` false)
  (set `CharacterMovementComponent.MaxWalkSpeed` (`self.DefaultSpeed`) (`self.CharacterMovement`)))

(fn `UserConstructionScript`)